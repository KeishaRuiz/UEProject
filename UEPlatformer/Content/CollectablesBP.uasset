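; Collectable pickup actor that counts down the level's remaining collectables.
; On any actor overlap it decrements CollectablesLeft in bpGameMode, shows a CollectableWidget and destroys itself.
; When the count reaches zero, it opens the map named "Level".
; A Sphere component toggles the actor's player input as a Character enters or leaves, though the graph defines no input events.
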(event `self.ReceiveActorBeginOverlap`
  (params (OtherActor :type "Actor Object Reference"))
  (bind _asbp_game_mode (cast `/Game/bpGameMode` (`GameplayStatics.GetGameMode`)))
  (bind _result (`/Engine/EditorBlueprintResources/StandardMacros.DecrementInt` (`/Game/bpGameMode.Collectables Left` _asbp_game_mode))
    (:`  `
      (set `/Game/bpGameMode.Collectables Left` _result _asbp_game_mode)
      (bind _returnvalue (`|CreateWidget` "/Game/CollectableWidget.CollectableWidget_C"))
      (`UserWidget.AddToViewport` _returnvalue 0)
      (`self.K2_DestroyActor`)
      (bind _asbp_game_mode_2 (cast `/Game/bpGameMode` (`GameplayStatics.GetGameMode`)))
      (if (== 0 (`/Game/bpGameMode.Collectables Left` _asbp_game_mode_2))
        (`GameplayStatics.OpenLevel` "Level")))))

(event `self.Sphere.OnComponentBeginOverlap`
  (params (OverlappedComponent :type "PrimitiveComponent Object Reference") (OtherActor :type "Actor Object Reference") (OtherComp :type "PrimitiveComponent Object Reference") (OtherBodyIndex :type Integer) (bFromSweep :type Boolean) (SweepResult :type "HitResult Structure (by ref)"))
  (cast `Character` OtherActor)
  (`self.EnableInput` (`GameplayStatics.GetPlayerController` 0)))

(event `self.Sphere.OnComponentEndOverlap`
  (params (OverlappedComponent :type "PrimitiveComponent Object Reference") (OtherActor :type "Actor Object Reference") (OtherComp :type "PrimitiveComponent Object Reference") (OtherBodyIndex :type Integer))
  (cast `Character` OtherActor)
  (`self.DisableInput` (`GameplayStatics.GetPlayerController` 0)))

(fn `UserConstructionScript`)